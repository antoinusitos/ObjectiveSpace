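; Double sliding door Blueprint that animates two panels, L and R, apart and back together.
; BeginPlay caches both panels' relative start locations as the base for movement.
; PlayAnimation checks MyIsOpen to play one timeline forward or in reverse, offsetting the panels in opposite directions along local X.
; When the timeline finishes, it calls PostAnimation.
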(event EventPlayAnimation
  (if (Variables|Default|GetmyIsOpen)
    (bind _newtrack_0 (Timeline|Timeline_0 ReverseFromEnd)
      (:Update
        (Transformation|SetRelativeLocation (Variables|Default|Getl) (+ (Variables|Default|GetLStartPos) (Math|Vector|MakeVector (* _newtrack_0 -1.0) 0.0 0.0)) false false)
        (Transformation|SetRelativeLocation (Variables|Default|Getr) (+ (Variables|Default|GetRStartPos) (Math|Vector|MakeVector _newtrack_0 0.0 0.0)) false false))
      (:Finished
        (Class|OSStaticEntity|PostAnimation)))
    (else
      (Timeline|Timeline_0 PlayFromStart))))

(event EventBeginPlay
  (Variables|Default|SetLStartPos (Variables|/Script/Engine.SceneComponent|GetRelativeLocation (Variables|Default|Getl)))
  (Variables|Default|SetRStartPos (Variables|/Script/Engine.SceneComponent|GetRelativeLocation (Variables|Default|Getr))))

(fn ConstructionScript)