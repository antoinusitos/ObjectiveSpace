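; Player Blueprint that handles arms and rifle animation, weapon holstering and the bullet HUD.
; Thin events call functions that play paired montages on the arm mesh and child-actor weapon, then refresh the UI_OSPlayer widget.
; Reload refills ammo after a fixed delay rather than a montage notify.
; Holstering sets an arms AnimBP flag and uses delays to time mesh visibility and clear the switching lock.
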(event EventPlayAnimationFire
  (CallFunction|PlayAnimationFireFunc))

(event EventSpawnUI
  (CallFunction|SpawnUIFunc))

(event EventPlayAnimationReload
  (Utilities|PlayAnimationReloadFunc))

(event EventSetAnimationSprint
  (params (aNewState :type Boolean))
  (Variables|Default|SetIsSprinting aNewState))

(event EventShowInteractUI
  (params (aText :type String))
  (Default|ShowInteract (Variables|Default|GetPlayerUI) aText))

(event EventHolsterWeapon
  (params (aNewState :type Boolean))
  (Utilities|HolsterWeaponFunc aNewState))

(event EventBPUpdateWeaponUI
  (if (and (Utilities|IsValid (Variables|/Script/Engine.ChildActorComponent|GetChildActor (Variables|Default|GetmyChildActorComponent))) (not (Class|OSPlayer|GetWeaponIsHolstered)))
    (bind _asbp_osweapon (Utilities|Casting|CastToBP_OSWeapon (Variables|/Script/Engine.ChildActorComponent|GetChildActor (Variables|Default|GetmyChildActorComponent))))
    (Default|UpdateBullets (Variables|Default|GetPlayerUI) _asbp_osweapon)
    (else
      (Default|HideBullets (Variables|Default|GetPlayerUI)))))

(fn ConstructionScript)

(fn GetArmAnimBP
  (Utilities|IsValid (Variables|Default|GetArmAnimBP)
    (:Is%20Valid
      (return (Variables|Default|GetArmAnimBP)))
    (:Is%20Not%20Valid
      (bind _asbp_so_arms_anim_bp (Utilities|Casting|CastToBP_SO_Arms_AnimBP (Components|SkeletalMesh|GetAnimInstance (Variables|Default|GetmyArmMesh)))
        (:then
          (Variables|Default|SetArmAnimBP _asbp_so_arms_anim_bp)
          (return (Variables|Default|GetArmAnimBP)))
        (:CastFailed
          (Development|PrintString "FAIL"))))))

(fn PlayAnimationFireFunc
  (bind _myarmmesh (Variables|Default|GetmyArmMesh))
  (bind _returnvalue (Components|SkeletalMesh|GetAnimInstance _myarmmesh))
  (if (== (Math|Random|RandomIntegerinRange 1 2) 1)
    (Animation|Montage|MontagePlay _returnvalue "/Game/FPS_Assault_Pack/Animations/Rifle/A_Arms_Rifle_Shoot01_Montage.A_Arms_Rifle_Shoot01_Montage" 1.0 "MontageLength" 0.0 true)
    (else
      (Animation|Montage|MontagePlay _returnvalue "/Game/FPS_Assault_Pack/Animations/Rifle/A_Arms_Rifle_Shoot02_Montage.A_Arms_Rifle_Shoot02_Montage" 1.0 "MontageLength" 0.0 true)))
  (bind _asbp_osweapon (Utilities|Casting|CastToBP_OSWeapon (Variables|/Script/Engine.ChildActorComponent|GetChildActor (Variables|Default|GetmyChildActorComponent))))
  (Animation|Montage|MontagePlay (Components|SkeletalMesh|GetAnimInstance (Variables|/Script/Objective_Space.OSWeapon|GetmyWeaponMesh _asbp_osweapon)) "/Game/FPS_Assault_Pack/Animations/Rifle/A_Rifle_Shoot01_Montage.A_Rifle_Shoot01_Montage" 1.0 "MontageLength" 0.0 true)
  (Default|UpdateBullets (Variables|Default|GetPlayerUI) _asbp_osweapon))

(fn SpawnUIFunc
  (bind _returnvalue (UserInterface|CreateWidget "/Game/Assets/UI/UI_OSPlayer.UI_OSPlayer_C"))
  (bind _output_get (Variables|Default|SetPlayerUI _returnvalue))
  (UserInterface|Viewport|AddtoViewport _output_get 0)
  (bind _asbp_osweapon (Utilities|Casting|CastToBP_OSWeapon (Variables|/Script/Engine.ChildActorComponent|GetChildActor (Variables|Default|GetmyChildActorComponent))))
  (Default|UpdateBullets (Variables|Default|GetPlayerUI) _asbp_osweapon))